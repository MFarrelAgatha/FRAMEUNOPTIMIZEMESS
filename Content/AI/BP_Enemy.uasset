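; BP_Enemy is a melee enemy character with a sword combo and a big attack, both played as montages.
; Incoming damage lowers a stat in BPCStats, which receives the widget's health bar on BeginPlay.
; Begin/EndSwordTrace run a looping timer of sphere traces along the sword, throttled by DoOnce and Delay, while PointDamageTrace applies single-point radius hits.
; Die disables movement, ragdolls the mesh, hides the widget and stops sword damage.
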(event `self.ReceiveBeginPlay`
  (bind _aswb_enemy_health_1 (cast `/Game/UI/WB_EnemyHealth1` (`WidgetComponent.GetWidget` (`self.Widget`))))
  (`/Game/Blueprint/BPC_Stats.Set Health Progress bar` (`self.BPC_Stats`) (`/Game/UI/WB_EnemyHealth1.HealthBar` _aswb_enemy_health_1)))

(event `self.ReceiveAnyDamage`
  (params (Damage :type "Float (single-precision)") (DamageType :type "DamageType Object Reference") (InstigatedBy :type "Controller Object Reference") (DamageCauser :type "Actor Object Reference"))
  (`/Game/Blueprint/BPC_Stats.Increase Value` (`self.BPC_Stats`) "NewEnumerator0" (* Damage -1.0)))

(event `/Game/Blueprint/BPI_Damage.End Sword Trace`
  (if (`KismetSystemLibrary.K2_IsValidTimerHandle` (stale `/Game/Blueprint/BPI_Damage.Begin Sword Trace` _returnvalue))
    (`KismetSystemLibrary.K2_ClearAndInvalidateTimerHandle` (stale `/Game/Blueprint/BPI_Damage.Begin Sword Trace` _returnvalue))))

(event `/Game/Blueprint/BPI_Damage.Begin Sword Trace`
  (bind _returnvalue (`KismetSystemLibrary.K2_SetTimerDelegate` (delegate `Damege Trace`) 0.01 true)))

(event `Damege Trace`
  (if (not (`self.isDead`))
    (bind (_outhit _returnvalue) (`KismetSystemLibrary.SphereTraceSingleForObjects` :`Start` (`SceneComponent.K2_GetComponentLocation` (`self.Start Sword Trace pos`)) :`End` (`SceneComponent.K2_GetComponentLocation` (`self.END Sword Trace pos`)) :`Radius` 25.0 :`ObjectTypes` (`|MakeArray` "ObjectTypeQuery3" :!type "EObjectTypeQuery Enum") :`DrawDebugType` "ForOneFrame" :`DrawTime` 2.0))
    (if _returnvalue
      (`/Engine/EditorBlueprintResources/StandardMacros.DoOnce` false :!label _label
        (:`Completed`
          (`GameplayStatics.ApplyDamage` (`.HitActor` (`GameplayStatics.BreakHitResult` _outhit)) (`self.Sword Damage`))
          (`KismetSystemLibrary.Delay` 0.3)
          (goto _label :!via `Reset`))))))

(event `/Game/Blueprint/BPI_Damage.Die`
  (`CharacterMovementComponent.DisableMovement` (`self.CharacterMovement`))
  (`PrimitiveComponent.SetSimulatePhysics` (`self.Mesh`) true)
  (`SceneComponent.SetVisibility` (`self.Widget`) false false)
  (set `self.isDead` true))

(event `/Game/Blueprint/BPI_Damage.Point Damage Trace`
  (bind _returnvalue (`SceneComponent.K2_GetComponentLocation` (`self.Point Trace Pos`)))
  (bind (_outhit _returnvalue_2) (`KismetSystemLibrary.SphereTraceSingleForObjects` :`Start` _returnvalue :`End` _returnvalue :`Radius` (`self.pointAttackRadius`) :`ObjectTypes` (`|MakeArray` "ObjectTypeQuery3" :!type "EObjectTypeQuery Enum") :`DrawDebugType` "ForDuration"))
  (if _returnvalue_2
    (`GameplayStatics.ApplyDamage` (`.HitActor` (`GameplayStatics.BreakHitResult` _outhit)) 10.0)))

(fn `Big Attack`
  (returns (Duration :type "Float (double-precision)"))
  (bind _returnvalue (`self.PlayAnimMontage` "/Game/Characters/Souls/Combat/BigAttack_Montage.BigAttack_Montage"))
  (return _returnvalue))

(fn `SwordAttack`
  (returns (Duration :type "Float (double-precision)"))
  (bind _returnvalue (`self.PlayAnimMontage` "/Game/Characters/Souls/Combat/SwordAttackCombo_Montage.SwordAttackCombo_Montage"))
  (return _returnvalue))

(fn `UserConstructionScript`)